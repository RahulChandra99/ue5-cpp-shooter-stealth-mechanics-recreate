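; Master weapon pickup actor for the demo content that spins, shows info widgets and lets the first-person player pick it up.
; Overlap reveals animated name, info and interact widgets, slows the spin and enables Interact, which passes the actor to PlayerRef.PickUpWeapon.
; A reversible timeline blends inspection depth of field and vignette on the player's FPS and ADS cameras.
; OffAll shuts down rotation, overlaps and idle particles; outline toggles are empty stubs.
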(event OnComponentBeginOverlap(RootCol)
  (params (OverlappedComponent :type Primitive%20Component%20Object%20Reference) (OtherActor :type Actor%20Object%20Reference) (OtherComp :type Primitive%20Component%20Object%20Reference) (OtherBodyIndex :type Integer) (bFromSweep :type Boolean) (SweepResult :type Hit%20Result%20Structure%20%28by%20ref%29))
  ;[0.2344 0.2655 0.5] Overlap
  (CallFunction|SwitchonDoF)
  (CallFunction|DisplayWidgetInfo (Variables|itemSettings|GetWeaponName) (Variables|Default|GetWidget_ItemName) true)
  (CallFunction|DisplayWidgetInfo (Variables|itemSettings|GetWeaponInfo) (Variables|Default|GetWidget_itemInfo) true)
  (Rendering|SetVisibility (Variables|Default|GetWidget_Interact) true false)
  (CallFunction|PlayWidgetAnimation)
  (bind _asfirst_person_character (Utilities|Casting|CastToFirstPersonCharacter (Game|GetPlayerCharacter 0)))
  (Variables|Default|SetPlayerRef _asfirst_person_character)
  (Variables|ItemSettings|SetCanPickUp true)
  (Input|EnableInput (Game|GetPlayerController 0))
  (Variables|itemSettings|SetRotationSpeed 3e+01)
  (CallFunction|ToggleColoredOutline))

(event OnComponentEndOverlap(RootCol)
  (params (OverlappedComponent :type Primitive%20Component%20Object%20Reference) (OtherActor :type Actor%20Object%20Reference) (OtherComp :type Primitive%20Component%20Object%20Reference) (OtherBodyIndex :type Integer))
  ;[0.2344 0.2655 0.5] Overlap
  (CallFunction|SwitchOFFDoF)
  (CallFunction|DisplayWidgetInfo (Variables|itemSettings|GetWeaponName) (Variables|Default|GetWidget_ItemName) false)
  (CallFunction|DisplayWidgetInfo (Variables|itemSettings|GetWeaponInfo) (Variables|Default|GetWidget_itemInfo) false)
  (Rendering|SetVisibility (Variables|Default|GetWidget_Interact) false false)
  (Variables|ItemSettings|SetCanPickUp false)
  (CallFunction|ToggleBlackOutline)
  (Variables|itemSettings|SetRotationSpeed 9e+01))

(event Custom|OffAll
  ;[0.2344 0.2655 0.5] Interact
  (Rendering|SetVisibility (Variables|Default|GetWidget_ItemName) false false)
  (Variables|/Script/Engine.PrimitiveComponent|SetbGenerateOverlapEvents (Variables|Default|GetRootCol) false)
  (Variables|itemSettings|SetIsRotating false)
  (Variables|itemSettings|SetRotationSpeed 0.0)
  (CallFunction|ToggleBlackOutline)
  (CallFunction|SwitchOFFDoF)
  (Components|Activation|Deactivate (Variables|Default|GetWeapon_Idle_Particle)))

(event Custom|ToggleColoredOutline
  ;[0.2344 0.2655 0.5] Spin Object
)

(event Custom|ToggleBlackOutline
  ;[0.2344 0.2655 0.5] Spin Object
)

(event Custom|PlayWidgetAnimation
  ;[0.2344 0.2655 0.5] Display Widgets
  (Utilities|FlowControl|Sequence
    (:then_0
      (UserInterface|Animation|PlayAnimation (stale EventBeginPlay _aswidget_item_info) (Variables|/Game/VFX_SciFi_Muzzle_And_Impact_Pack_1/Example_Content/DemoContent/Blueprints/Widgets/Widget_item_Info.Widget_item_Info_C|GetAppear (stale EventBeginPlay _aswidget_item_info)) 0.0 1 "Forward" 1.0 false))
    (:then_1
      (UserInterface|Animation|PlayAnimation (stale EventBeginPlay _aswidget_item_name) (Variables|/Game/VFX_SciFi_Muzzle_And_Impact_Pack_1/Example_Content/DemoContent/Blueprints/Widgets/Widget_item_name.Widget_item_name_C|GetAppear (stale EventBeginPlay _aswidget_item_name)) 0.0 1 "Forward" 1.0 false))
    (:then_2
      (UserInterface|Animation|PlayAnimation (stale EventBeginPlay _aswidget_interact) (Variables|/Game/VFX_SciFi_Muzzle_And_Impact_Pack_1/Example_Content/DemoContent/Blueprints/Widgets/Widget_Interact.Widget_Interact_C|GetAppear (stale EventBeginPlay _aswidget_interact)) 0.0 1 "Forward" 1.0 false)
      (Utilities|FlowControl|Delay 0.8)
      (UserInterface|Animation|PlayAnimation (stale EventBeginPlay _aswidget_interact) (Variables|/Game/VFX_SciFi_Muzzle_And_Impact_Pack_1/Example_Content/DemoContent/Blueprints/Widgets/Widget_Interact.Widget_Interact_C|GetBouncing_Loop (stale EventBeginPlay _aswidget_interact)) 0.0 0 "Forward" 1.0 false))))

(event Custom|SwitchOn_DoF
  ;[0.2344 0.2655 0.5] Display Widgets
  (|InspectionDepthofField))

(event Custom|SwitchOFF_DoF
  ;[0.2344 0.2655 0.5] Display Widgets
  (|InspectionDepthofField) ; enters at Reverse
)

(event EventBeginPlay
  (Utilities|FlowControl|Sequence
    (:then_0
      ;[0.2344 0.2655 0.5] Display Widgets
      (Utilities|FlowControl|Sequence
        (:then_0
          (bind _aswidget_item_info (Utilities|Casting|CastToWidget_item_Info (UserInterface|GetUserWidgetObject (Variables|Default|GetWidget_itemInfo))))
          (Variables|/Game/VFX_SciFi_Muzzle_And_Impact_Pack_1/Example_Content/DemoContent/Blueprints/Widgets/Widget_item_Info.Widget_item_Info_C|SetInfo _aswidget_item_info (Variables|itemSettings|GetWeaponInfo)))
        (:then_1
          (bind _aswidget_item_name (Utilities|Casting|CastToWidget_item_name (UserInterface|GetUserWidgetObject (Variables|Default|GetWidget_ItemName))))
          (Variables|/Game/VFX_SciFi_Muzzle_And_Impact_Pack_1/Example_Content/DemoContent/Blueprints/Widgets/Widget_item_name.Widget_item_name_C|Setname _aswidget_item_name (Variables|itemSettings|GetWeaponName)))
        (:then_2
          (bind _aswidget_interact (Utilities|Casting|CastToWidget_Interact (UserInterface|GetUserWidgetObject (Variables|Default|GetWidget_Interact)))))))
    (:then_1
      (Variables|itemSettings|SetRotationSpeed 9e+01))))

(event EventTick
  (params (DeltaSeconds :type Float%20%28single-precision%29))
  ;[0.2344 0.2655 0.5] Spin Object
  (if (Variables|itemSettings|GetIsRotating)
    (Transformation|AddRelativeRotation (Variables|Default|GetRoot_Rotation) (* (Math|Rotator|MakeRotator 0.0 0.0 (Variables|itemSettings|GetRotationSpeed)) DeltaSeconds) false false)))

(event Input|ActionEvents|InputActionInteract
  (params (Key :type Key%20Structure))
  ;[0.2344 0.2655 0.5] Interact
  (:Pressed
    (if (Variables|ItemSettings|GetCanPickUp)
      (Default|PickUpWeapon (Variables|Default|GetPlayerRef) self))))

(fn ConstructionScript)

(fn DisplayWidgetInfo
  (params (Name :type Text) (NewParam :type Widget%20Component%20Object%20Reference) (ShouldBeVisible? :type Boolean))
  (Rendering|SetVisibility NewParam (and (not (Utilities|Text|TextIsEmpty Name)) ShouldBeVisible?) false))